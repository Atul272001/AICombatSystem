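; BP_EnemyCharacter is an enemy character Blueprint that shows its health on a world-space health bar widget.
; On BeginPlay it binds to the HealthComponent's health-change event, caches the WBP_HealthBar widget and initializes the bar from max health.
; Health changes are forwarded to the widget's UpdateHealth function.
; Every Tick, the widget component rotates to face the player camera.
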(event `self.ReceiveBeginPlay`
  (`parent.ReceiveBeginPlay`)
  (add `HealthComponent.OnHealthChanged` (`self.HealthComponent`) (delegate `ChangeHealth`))
  (bind _aswbp_health_bar (cast `/Game/UI/WBP_HealthBar` (`WidgetComponent.GetUserWidgetObject` (`self.HealthBarWidget`))))
  (bind _output_get (set `self.HealthBarWidgetRef` _aswbp_health_bar))
  (`ProgressBar.SetPercent` (`/Game/UI/WBP_HealthBar.HealthBar` _output_get) (`HealthComponent.GetMaxHealth` (`self.HealthComponent`))))

(event `ChangeHealth`
  (params (CurrentHealth :type "Float (single-precision)") (MaxHealth :type "Float (single-precision)"))
  (bind _healthbarwidgetref (`self.HealthBarWidgetRef`)
    (:`then`
      (`/Game/UI/WBP_HealthBar.UpdateHealth` _healthbarwidgetref CurrentHealth MaxHealth))
    (:`else`)))

(event `self.ReceiveTick`
  (params (DeltaSeconds :type "Float (single-precision)"))
  (`SceneComponent.K2_SetWorldRotation` (`self.HealthBarWidget`) (`KismetMathLibrary.FindLookAtRotation` (`SceneComponent.K2_GetComponentLocation` (`self.HealthBarWidget`)) (`PlayerCameraManager.GetCameraLocation` (`GameplayStatics.GetPlayerCameraManager` 0))) false false))

(fn `UserConstructionScript`)